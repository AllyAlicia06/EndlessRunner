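; Floor tile for a three-lane endless runner that asks the game mode for a new floor and destroys itself when the player overlaps its DestroyBox.
; Spawn events add obstacles, platforms, coin rows and environment pieces as child actors at lane or start points.
; Platforms shift along X so their arrow component meets the tile's AttachPoint.
; Coins use a vertical line trace to sit just above the surface beneath them.
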(event `self.Destroy Box.OnComponentBeginOverlap`
  (params (OverlappedComponent :type "PrimitiveComponent Object Reference") (OtherActor :type "Actor Object Reference") (OtherComp :type "PrimitiveComponent Object Reference") (OtherBodyIndex :type Integer) (bFromSweep :type Boolean) (SweepResult :type "HitResult Structure (by ref)"))
  ; Add/Destroy Floor
  (if (== OtherActor (`GameplayStatics.GetPlayerCharacter` 0))
    (message `/Game/BPInterfaces/GameModeBPInterface.Add New Floor` (`GameplayStatics.GetGameMode`))
    (`self.K2_DestroyActor`)))

(event `Spawn Obstacle`
  (params (`Obstacle Class` :type "/Game/Blueprints/Obstacles/BaseObstacle_BP Class Reference") (`Lane No` :type Integer))
  ; Spawn Random Obstacles
  (bind _returnvalue (`AddComponent|NODE_AddChildActorComponent-0` :`RelativeTransform` (`KismetMathLibrary.MakeTransform` (`SceneComponent.RelativeLocation` (select `int` `Lane No` :`0` (`self.Spawn Point1`) :`1` (`self.Spawn Point2`) :`2` (`self.Spawn Point3`))))))
  (`ChildActorComponent.SetChildActorClass` _returnvalue `Obstacle Class`))

(event `Spawn Platform`
  (params (`Platform Class` :type "/Game/Blueprints/Platforms/BasePlatform_BP Class Reference") (`Lane No` :type Integer))
  (bind _returnvalue_x (`KismetMathLibrary.BreakVector` (`SceneComponent.K2_GetComponentLocation` (`self.AttachPoint`))))
  ; Spawn Random Platforms
  (bind _returnvalue (`AddComponent|NODE_AddChildActorComponent-1` :`RelativeTransform` (`KismetMathLibrary.MakeTransform` (`SceneComponent.RelativeLocation` (select `int` `Lane No` :`0` (`self.Spawn Point1`) :`1` (`self.Spawn Point2`) :`2` (`self.Spawn Point3`))))))
  (`ChildActorComponent.SetChildActorClass` _returnvalue `Platform Class`)
  (bind _returnvalue_x_2 (`KismetMathLibrary.BreakVector` (`SceneComponent.K2_GetComponentLocation` (`self.GetComponentByClass` (`ChildActorComponent.ChildActor` _returnvalue) "/Script/Engine.ArrowComponent"))))
  (bind (_returnvalue_x_3 _returnvalue_y _returnvalue_z) (`KismetMathLibrary.BreakVector` (`SceneComponent.K2_GetComponentLocation` _returnvalue)))
  ; Stick Platform End Point to Road's End Point
  (`SceneComponent.K2_SetWorldLocation` _returnvalue (`KismetMathLibrary.MakeVector` (+ (- _returnvalue_x _returnvalue_x_2) _returnvalue_x_3) _returnvalue_y _returnvalue_z) false false))

(event `Spawn Coin`
  (params (Length :type Integer) (`Lane No` :type Integer))
  (for _index (range 1 (+ Length 1))
    (bind _returnvalue (`AddComponent|NODE_AddChildActorComponent-2` :`RelativeTransform` (`KismetMathLibrary.MakeTransform` (`KismetMathLibrary.MakeVector` (+ (- (.x (`SceneComponent.RelativeLocation` (select `int` `Lane No` :`0` (`self.Spawn Point1`) :`1` (`self.Spawn Point2`) :`2` (`self.Spawn Point3`)))) 400.0) (* _index 150)) (.y (`SceneComponent.RelativeLocation` (select `int` `Lane No` :`0` (`self.Spawn Point1`) :`1` (`self.Spawn Point2`) :`2` (`self.Spawn Point3`)))) 50.0))))
    (`ChildActorComponent.SetChildActorClass` _returnvalue "/Game/Blueprints/Currency/Coin_BP.Coin_BP_C")
    (`SceneComponent.K2_SetWorldLocation` _returnvalue (`self.Get Coin Spawning Height` (`SceneComponent.K2_GetComponentLocation` _returnvalue)) false false)))

(event `Spawn Environment`
  (params (`Environment Class` :type "/Game/Blueprints/Environment/BaseEnvironment_BP Class Reference"))
  (bind _returnvalue (`AddComponent|NODE_AddChildActorComponent-3` :`RelativeTransform` (`KismetMathLibrary.MakeTransform` (`SceneComponent.RelativeLocation` (`self.StartPoint`)))))
  (`ChildActorComponent.SetChildActorClass` _returnvalue `Environment Class`))

(fn `Get Coin Spawning Height`
  (params (`Coin Location` :type "Vector Structure"))
  (returns (`Spawn Location` :type "Vector Structure"))
  (bind _x (.x `Coin Location`))
  (bind _y (.y `Coin Location`))
  (bind (_outhit _returnvalue) (`KismetSystemLibrary.LineTraceSingle` :`Start` (`KismetMathLibrary.MakeVector` _x _y 1000.0) :`End` (`KismetMathLibrary.MakeVector` _x _y -1.0) :`TraceChannel` "TraceTypeQuery1" :`bIgnoreSelf` false))
  (if _returnvalue
    (return (`KismetMathLibrary.MakeVector` (.x (`.ImpactPoint` (`GameplayStatics.BreakHitResult` _outhit))) (.y (`.ImpactPoint` (`GameplayStatics.BreakHitResult` _outhit))) (+ (.z (`.ImpactPoint` (`GameplayStatics.BreakHitResult` _outhit))) 50.0)))))

(fn `UserConstructionScript`)