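; Base platform that builds itself at a random length from a ladder mesh and can kill the player on side impacts.
; Construction chains 4–7 mesh segments socket to socket, moves AttachPoint to the end, and centers and stretches DeathBox along the span in X.
; DeathBox hits check the normal's Y sign against the player's jump or roll montage, then send DeathMessage and apply a Y impulse to the mesh.
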(event `self.DeathBox.OnComponentHit`
  (params (HitComponent :type "PrimitiveComponent Object Reference") (OtherActor :type "Actor Object Reference") (OtherComp :type "PrimitiveComponent Object Reference") (NormalImpulse :type "Vector Structure") (Hit :type "HitResult Structure (by ref)"))
  (bind _returnvalue (`GameplayStatics.GetPlayerCharacter` 0))
  (bind _returnvalue_2 (`GameplayStatics.GetPlayerCharacter` 0))
  (bind _returnvalue_3 (`Character.GetCurrentMontage` _returnvalue))
  (bind _returnvalue_4 (`KismetMathLibrary.Round` (.y (`.Normal` (`GameplayStatics.BreakHitResult` Hit)))))
  (if (== OtherActor _returnvalue)
    (switch `int` _returnvalue_4
      (:`-1`
        (if (or (== _returnvalue_3 "/Game/Animations/SideJump/M_Neutral_Jump_LL_Start_Rfoot_Montage.M_Neutral_Jump_LL_Start_Rfoot_Montage") (== _returnvalue_3 "/Game/Animations/Roll/M_Neutral_Jump_F_Land_Roll_Lfoot_Montage.M_Neutral_Jump_F_Land_Roll_Lfoot_Montage"))
          (message `/Game/BPInterfaces/CharacterBPInterface.Death` _returnvalue_2 :!label _label)
          (`PrimitiveComponent.AddImpulse` (`Character.Mesh` _returnvalue_2) (`KismetMathLibrary.MakeVector` 0.0 (`KismetMathLibrary.Conv_IntToDouble` (* _returnvalue_4 -1000))) "None" false)))
      (:`1`
        (if (or (== _returnvalue_3 "/Game/Animations/SideJump/M_Neutral_Jump_RL_Start_Lfoot_Montage.M_Neutral_Jump_RL_Start_Lfoot_Montage") (== _returnvalue_3 "/Game/Animations/Roll/M_Neutral_Jump_F_Land_Roll_Lfoot_Montage.M_Neutral_Jump_F_Land_Roll_Lfoot_Montage"))
          (goto _label))))))

(fn `UserConstructionScript`
  (bind _deathbox (`self.DeathBox`))
  (bind _deathbox_2 (`self.DeathBox`))
  (bind (_returnvalue_x _returnvalue_y _returnvalue_z) (`KismetMathLibrary.BreakVector` (`SceneComponent.K2_GetComponentLocation` _deathbox_2)))
  (bind (_boxextent_x _boxextent_y _boxextent_z) (`KismetMathLibrary.BreakVector` (`BoxComponent.BoxExtent` _deathbox)))
  (`SceneComponent.K2_SetWorldLocation` (`self.Platform Mesh`) (`SceneComponent.GetSocketLocation` (`self.Ladder Mesh`) "AttachPoint") false false)
  (set `self.Last Platform Attach Point` (`SceneComponent.GetSocketLocation` (`self.Platform Mesh`) "AttachPoint"))
  (set `self.Platform Length` (`KismetMathLibrary.RandomIntegerInRange` 4 7))
  (for _ (range 1 (`self.Platform Length`))
    (bind _returnvalue (`AddComponent|NODE_AddStaticMeshComponent-0`))
    (`StaticMeshComponent.SetStaticMesh` _returnvalue (`StaticMeshComponent.StaticMesh` (`self.Platform Mesh`)))
    (`SceneComponent.K2_SetWorldLocation` _returnvalue (`self.Last Platform Attach Point`) false false)
    (set `self.Last Platform Attach Point` (`SceneComponent.GetSocketLocation` _returnvalue "AttachPoint"))
    (`PrimitiveComponent.SetCollisionResponseToChannel` _returnvalue "ECC_Camera" "ECR_Ignore")
    (`SceneComponent.K2_SetWorldLocation` (`self.AttachPoint`) (`self.Last Platform Attach Point`) false false))
  (`SceneComponent.K2_SetWorldLocation` _deathbox_2 (`KismetMathLibrary.MakeVector` (/ (.x (+ (`self.Last Platform Attach Point`) (`SceneComponent.GetSocketLocation` (`self.Ladder Mesh`) "AttachPoint"))) 2.0) _returnvalue_y _returnvalue_z) false false)
  (`BoxComponent.SetBoxExtent` _deathbox (`KismetMathLibrary.MakeVector` (/ (.x (- (`self.Last Platform Attach Point`) (`SceneComponent.GetSocketLocation` (`self.Ladder Mesh`) "AttachPoint"))) 2.0) _boxextent_y _boxextent_z) true))